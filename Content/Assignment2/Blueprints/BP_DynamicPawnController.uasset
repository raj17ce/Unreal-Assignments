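; BP_DynamicPawnController is a controller Blueprint that prints a pawn's attributes as debug text.
; Its DisplayAttributes event takes a PawnAttributes input and prints labeled Speed, Health and Jump Height values through separate PrintString calls.
; BeginPlay, Tick and the construction script are empty, so the Blueprint shows output only when that event is called.
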(event EventBeginPlay)

(event EventTick
  (params (DeltaSeconds :type Float%20%28single-precision%29)))

(event EventDisplayAttributes
  (params (PawnAttributes :type Pawn%20Attribute%20Asset%20Object%20Reference))
  (Development|PrintString (Utilities|String|Append "Speed : " (Utilities|String|ToString(Float) (Variables|/Script/Assignment2.PawnAttributeAsset|GetSpeed PawnAttributes))))
  (Development|PrintString (Utilities|String|Append "Health : " (Utilities|String|ToString(Float) (Variables|/Script/Assignment2.PawnAttributeAsset|GetHealth PawnAttributes))))
  (Development|PrintString (Utilities|String|Append "Jump Height : " (Utilities|String|ToString(Float) (Variables|/Script/Assignment2.PawnAttributeAsset|GetJumpHeight PawnAttributes)))))

(fn ConstructionScript)